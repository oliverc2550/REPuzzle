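; BP_LoweringDoor is a puzzle door that lowers when its linked puzzle object reports it has been solved.
; On BeginPlay it binds LowerDoor to that object's solved delegate, which plays a timeline lerping the actor from StartingLocation to EndingLocation.
; The construction script slows the timeline's play rate, and two editor helper functions capture the actor's current position as the start or end location.
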(event Custom|LowerDoor
  (bind _alpha (Timeline|LowerDoorTimeline PlayFromStart)
    (:Update
      (Transformation|SetActorLocation (Math|Vector|Lerp(Vector) (Variables|Default|GetStartingLocation) (Variables|Default|GetEndingLocation) _alpha) false false))))

(event EventBeginPlay
  (EventDispatchers|BindEventtoPuzzleHasBeenSolvedDelegate (Variables|Default|GetLinkedPuzzleObject) (delegate Custom|LowerDoor)))

(fn ConstructionScript
  (Components|Timeline|SetPlayRate (Variables|Default|GetLowerDoorTimeline) 0.33))

(fn EDITORSetStartingLocation
  (Variables|Default|SetStartingLocation (Transformation|GetActorLocation)))

(fn EDITORSetEndingLocation
  (Variables|Default|SetEndingLocation (Transformation|GetActorLocation)))